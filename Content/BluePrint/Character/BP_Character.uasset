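; BP_Character is a sprite-based combat character with health, faction-filtered melee hits, stun and defeat states.
; Hitbox overlaps damage opposing characters and briefly freeze the victim through CustomTimeDilation as hit stop.
; ReceiveAttack interrupts animation, then either jumps to defeat and disables capsule collision, or starts timed stun and shake timers.
; ShakeSprite alternates X offsets from the sprite's base location, but applies them to HitBox rather than Sprite.
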(event `self.ReceiveBeginPlay`
  (`self.Set Hitbox Collision` false)
  (set `self.Health` (`self.MaxHealth`))
  (set `self.SpriteBaseLocation` (`SceneComponent.RelativeLocation` (`self.Sprite`))))

(event `HItStopSequence`
  (params (Duration :type "Float (single-precision)" :default 0.3))
  (set `self.CustomTimeDilation` 0.0)
  (`KismetSystemLibrary.RetriggerableDelay` Duration)
  (set `self.CustomTimeDilation` 1.0))

(event `self.HitBox.OnComponentBeginOverlap`
  (params (OverlappedComponent :type "PrimitiveComponent Object Reference") (OtherActor :type "Actor Object Reference") (OtherComp :type "PrimitiveComponent Object Reference") (OtherBodyIndex :type Integer) (bFromSweep :type Boolean) (SweepResult :type "HitResult Structure (by ref)"))
  (bind _asbp_character (cast `/Game/BluePrint/Character/BP_Character` OtherActor))
  (if (!= (`/Game/BluePrint/Character/BP_Character.Faction` _asbp_character) (`self.Faction`))
    (`self.ReceiveAttack` _asbp_character 25.0)
    (`self.HItStopSequence` _asbp_character 0.2)))

(event `ShakeSprite`
  (bind (_spritebaselocation_x _spritebaselocation_y _spritebaselocation_z) (`KismetMathLibrary.BreakVector` (`self.SpriteBaseLocation`)))
  (bind _isa (`/Engine/EditorBlueprintResources/StandardMacros.FlipFlop`)
    (:`A`
      _)
    (:`B`
      _))
  (`SceneComponent.K2_SetRelativeLocation` (`self.HitBox`) (`KismetMathLibrary.MakeVector` (+ _spritebaselocation_x (select `bool` _isa :`false` (* (`self.SpriteShakeDistance`) -1.0) :`true` (`self.SpriteShakeDistance`))) _spritebaselocation_y _spritebaselocation_z) false false))

(fn `CanAct`
  (returns (CanAct :type Boolean))
  (return (and (not (`self.isAttacking`)) (not (`self.isStunned`)) (not (`self.isDefeated`)))))

(fn `ClearStun`
  (bind _output_get (set `self.isStunned` false))
  (`self.StunStateChanger` _output_get)
  (`KismetSystemLibrary.K2_ClearAndInvalidateTimerHandle` (`self.SpriteShakeHandle`)))

(fn `ReceiveAttack`
  (params (Damage :type "Float (double-precision)" :default 25.0))
  (if (not (`self.isDefeated`))
    (`GameplayStatics.PlaySoundAtLocation` null (`self.K2_GetActorLocation`) (struct) 1.0 1.0 0.0 null null null null)
    (set `self.Health` (- (`self.Health`) (`local.Damage`)))
    (`PaperZDAnimInstance.StopAllAnimationOverrides` (`self.GetAnimInstance`))
    (if (<= (`self.Health`) 0.0)
      (`PaperZDAnimInstance.JumpToNode` (`self.GetAnimInstance`) "JumpDefeated" "None")
      (set `self.isDefeated` true)
      (`PrimitiveComponent.SetCollisionEnabled` (`self.CapsuleComponent`) "NoCollision")
      (else
        (bind _output_get (set `self.isStunned` true))
        (`self.StunStateChanger` _output_get)
        (`PaperZDAnimInstance.JumpToNode` (`self.GetAnimInstance`) "JumpStunned" "None")
        (`KismetSystemLibrary.K2_SetTimerDelegate` (`|CreateDelegate` :!event `ClearStun`) (`self.StunLength`))
        (bind _returnvalue (`KismetSystemLibrary.K2_SetTimerDelegate` (`|CreateDelegate` :!event `ShakeSprite`) 0.05 true))
        (set `self.SpriteShakeHandle` _returnvalue)))))

(fn `Set Hitbox Collision`
  (params (SetHitBox :type Boolean))
  (if SetHitBox
    (`PrimitiveComponent.SetCollisionEnabled` (`self.HitBox`) "QueryOnly")
    (else
      (`PrimitiveComponent.SetCollisionEnabled` (`self.HitBox`) "NoCollision"))))

(fn `UserConstructionScript`)