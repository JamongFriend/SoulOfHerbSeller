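; GM_Platformer is a game mode that runs a quick-draw duel between the Player and Glass.
; Tick moves Intro to Wait after a start time, then a random Delay switches to Draw, broadcasts the phase start and shows the BP_Exclamation cue.
; QDSuccessfully defeats Glass or Player by its condition, hides the cue and starts a one-shot timer.
; QDReset restores Intro and both duelists, while QDFinished ends the round.
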(event `self.ReceiveBeginPlay`
  (bind _returnvalue (`GameplayStatics.GetActorOfClass` "/Game/BluePrint/QuickDraw/BP_Exclamation.BP_Exclamation_C"))
  (set `self.ExclamationRef` _returnvalue))

(event `self.ReceiveTick`
  (params (DeltaSeconds :type "Float (single-precision)"))
  (set `self.ElapseTime` (+ DeltaSeconds (`self.ElapseTime`)))
  (switch `/Game/BluePrint/QuickDraw/E_QDM_Phase` (`self.Phase`)
    (:`NewEnumerator0`
      (if (>= (`self.ElapseTime`) (`self.RoundStartTime`))
        (set `self.Phase` "NewEnumerator1")
        (`KismetSystemLibrary.Delay` (`KismetMathLibrary.RandomFloatInRange` (`self.MinDrawDelay`) (`self.MaxDrawDelay`)))
        (set `self.Phase` "NewEnumerator2")
        (`self.DrawPhaseStarted`)
        (`/Engine/EditorBlueprintResources/StandardMacros.IsValid` (`self.ExclamationRef`)
          (:`Is Valid`
            (`/Game/BluePrint/QuickDraw/BP_Exclamation.SetVisibility` (`self.ExclamationRef`) true))
          (:`Is Not Valid`
            (`KismetSystemLibrary.PrintString` "Exclamation not found")))))))

(fn `QD_finished`
  (set `self.Phase` "NewEnumerator3"))

(fn `QD_Reset`
  (set `self.Phase` "NewEnumerator0")
  (set `self.ElapseTime` 0.0)
  (`/Game/BluePrint/QuickDraw/BP_QuickDraw.reset` (`self.Player`))
  (`/Game/BluePrint/QuickDraw/BP_QuickDraw.reset` (`self.Glass`)))

(fn `QD_Successfully`
  (params (Condition :type Boolean))
  (if Condition
    (`/Game/BluePrint/QuickDraw/BP_QuickDraw.Defeated` (`self.Glass`))
    (else
      (`/Game/BluePrint/QuickDraw/BP_QuickDraw.Defeated` (`self.player`))))
  (`/Engine/EditorBlueprintResources/StandardMacros.IsValid` (`self.ExclamationRef`)
    (:`Is Valid`
      (`/Game/BluePrint/QuickDraw/BP_Exclamation.SetVisibility` (`self.ExclamationRef`) false)
      (`KismetSystemLibrary.K2_SetTimerDelegate` (`|CreateDelegate` :!event `QD_Reset`) (`self.Out`)))))

(fn `UserConstructionScript`)