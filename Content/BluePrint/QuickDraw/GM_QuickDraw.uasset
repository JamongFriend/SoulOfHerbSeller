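; Game mode for a quick-draw duel between the player and a Grass opponent, run as a phase state machine.
; Tick moves Intro to Wait after a start time, then after a random delay enters Draw, calls DrawPhaseStarted and shows the exclamation cue.
; Successfully defeats the losing side, hides the cue and starts a one-shot timer.
; Reset restores Intro and both duelists, and Finished sets the end phase.
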(event `self.ReceiveBeginPlay`
  (bind _returnvalue (`GameplayStatics.GetActorOfClass` "/Game/BluePrint/QuickDraw/BP_Exclamation.BP_Exclamation_C"))
  (set `self.ExclamationRef` _returnvalue)
  (bind _returnvalue_2 (`GameplayStatics.GetActorOfClass` "/Game/BluePrint/QuickDraw/BP_QD_Player.BP_QD_Player_C"))
  (set `self.Player` _returnvalue_2)
  (bind _returnvalue_3 (`GameplayStatics.GetActorOfClass` "/Game/BluePrint/QuickDraw/BP_QD_Grass.BP_QD_Grass_C"))
  (set `self.Glass` _returnvalue_3))

(event `self.ReceiveTick`
  (params (DeltaSeconds :type "Float (single-precision)"))
  (set `self.ElapseTime` (+ DeltaSeconds (`self.ElapseTime`)))
  (switch `/Game/BluePrint/QuickDraw/E_QDM_Phase` (`self.Phase`)
    (:`NewEnumerator0`
      (if (>= (`self.ElapseTime`) (`self.RoundStartTime`))
        (set `self.Phase` "NewEnumerator1")
        (`KismetSystemLibrary.Delay` (`KismetMathLibrary.RandomFloatInRange` (`self.MinDrawDelay`) (`self.MaxDrawDelay`)))
        (set `self.Phase` "NewEnumerator2")
        (`self.DrawPhaseStarted`)
        (`/Engine/EditorBlueprintResources/StandardMacros.IsValid` (`self.ExclamationRef`)
          (:`Is Valid`
            (`/Game/BluePrint/QuickDraw/BP_Exclamation.SetVisibility` (`self.ExclamationRef`) true)))))))

(fn `Finished`
  (set `self.Phase` "NewEnumerator3"))

(fn `Reset`
  (set `self.Phase` "NewEnumerator0")
  (set `self.ElapseTime` 0.0)
  (`/Game/BluePrint/QuickDraw/BP_QuickDraw.reset` (`self.Player`))
  (`/Game/BluePrint/QuickDraw/BP_QuickDraw.reset` (`self.Glass`)))

(fn `Successfully`
  (params (`Is Player` :type Boolean))
  (bind _exclamationref (`self.ExclamationRef`))
  (if `Is Player`
    (`/Game/BluePrint/QuickDraw/BP_QuickDraw.Defeated` (`self.Glass`))
    (else
      (`/Game/BluePrint/QuickDraw/BP_QuickDraw.Defeated` (`self.Player`))))
  (`/Engine/EditorBlueprintResources/StandardMacros.IsValid` _exclamationref
    (:`Is Valid`
      (`/Game/BluePrint/QuickDraw/BP_Exclamation.SetVisibility` _exclamationref false)
      (`KismetSystemLibrary.K2_SetTimerDelegate` (`|CreateDelegate` :!event `Reset`) (`self.Out`)))))

(fn `UserConstructionScript`)