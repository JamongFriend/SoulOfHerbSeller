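; BP_QD_Grass is a QuickDraw Blueprint named for grass that responds to the game mode's draw phase.
; On BeginPlay it runs the parent logic, then binds a handler to the game mode's DrawPhaseStarted event.
; When that phase starts, it waits for a configurable Delay and then calls QuickDraw.
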(event `self.ReceiveBeginPlay`
  (`parent.ReceiveBeginPlay`)
  (if true
    (add `/Game/BluePrint/QuickDraw/GM_QuickDraw.DrawPhaseStarted` (`self.Gamemode`) (delegate `OnDrawPhaseStarted`))
    (else
      (`KismetSystemLibrary.PrintString` "None GM"))))

(event `OnDrawPhaseStarted`
  (`KismetSystemLibrary.Delay` (`self.Delay`))
  (`self.QuickDraw`))

(fn `UserConstructionScript`
  (`parent.UserConstructionScript`))