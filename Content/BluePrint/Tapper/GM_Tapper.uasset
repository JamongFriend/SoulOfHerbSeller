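; GM_Tapper is the game mode for a tapper race, handling its start, winner announcement and exit.
; On BeginPlay it caches the BP_Tapper actor as Player, then broadcasts RaceStart after a short countdown delay.
; AnnounceWinner uses the IsRaceOver flag to fire only once, broadcasting AnnouncedWinner and setting a brief one-shot timer.
; A separate Finish function loads Map_2D to leave the race.
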(event `self.ReceiveBeginPlay`
  (`|ExecutionSequence`
    (:`then_0`
      (bind _returnvalue (`GameplayStatics.GetActorOfClass` "/Game/BluePrint/Tapper/BP_Tapper.BP_Tapper_C"))
      (set `self.Player` _returnvalue))
    (:`then_1`
      (`KismetSystemLibrary.Delay` 3.0)
      (`KismetSystemLibrary.PrintString` "Race Start")
      (`self.RaceStart`))))

(fn `AnnounceWinner`
  (if (not (`self.isRaceOver`))
    (set `self.isRaceOver` true)
    (`KismetSystemLibrary.PrintString` "Win!")
    (`self.AnnouncedWinner`)
    (`KismetSystemLibrary.K2_SetTimerDelegate` (`|CreateDelegate` :!event `Finish`) 2.0)))

(fn `Finish`
  (`GameplayStatics.OpenLevel` "Map_2D"))

(fn `UserConstructionScript`)