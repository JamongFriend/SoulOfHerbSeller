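; BP_Tapper_Player is the player Blueprint for the Tapper game, handling input, camera and UI setup when play begins.
; On BeginPlay it casts its controller to PlayerController and adds the IMC_Tapper Enhanced Input mapping context.
; It then switches the view to a CameraActor found in the level and adds the WB_Tapper widget to the viewport.
; It contains no input handlers or tick logic.
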(event `self.ReceiveBeginPlay`
  (`parent.ReceiveBeginPlay`)
  (bind _asplayer_controller (cast `PlayerController` (`self.GetController`)))
  (message `EnhancedInputSubsystemInterface.AddMappingContext` (pcsubsystem `EnhancedInputLocalPlayerSubsystem` _asplayer_controller) "/Game/input/IMC_Tapper.IMC_Tapper" 0 (struct))
  (bind _returnvalue (`GameplayStatics.GetActorOfClass` "/Script/Engine.CameraActor"))
  (`PlayerController.SetViewTargetWithBlend` (`GameplayStatics.GetPlayerController` 0) _returnvalue 0.0 "VTBlend_Linear" 0.0 false)
  (bind _returnvalue_2 (`|CreateWidget` "/Game/BluePrint/Tapper/WB_Tapper.WB_Tapper_C" (`GameplayStatics.GetPlayerController` 0)))
  (`UserWidget.AddToViewport` _returnvalue_2 0))

(fn `UserConstructionScript`
  (`parent.UserConstructionScript`))