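; BP_Tapper_Child is the player-controlled child Blueprint for the Tapper game, turning Enhanced Input presses into tap actions.
; On BeginPlay it runs the parent logic, adds the IMC_Tapper mapping context, switches the view to a CameraActor found in the level and shows the WB_Tapper widget.
; When IA_Tapper starts, it calls Tapper, whose logic is not defined in this Blueprint.
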(event `self.ReceiveBeginPlay`
  (bind _returnvalue (`GameplayStatics.GetPlayerController` 0))
  (`parent.ReceiveBeginPlay`)
  (bind _asplayer_controller (cast `PlayerController` (`self.GetController`)))
  (message `EnhancedInputSubsystemInterface.AddMappingContext` (pcsubsystem `EnhancedInputLocalPlayerSubsystem` _asplayer_controller) "/Game/input/IMC_Tapper.IMC_Tapper" 0 (struct))
  (bind _returnvalue_2 (`GameplayStatics.GetActorOfClass` "/Script/Engine.CameraActor"))
  (`PlayerController.SetViewTargetWithBlend` _returnvalue _returnvalue_2 0.0 "VTBlend_Linear" 0.0 false)
  (bind _returnvalue_3 (`|CreateWidget` "/Game/BluePrint/Tapper/WB_Tapper.WB_Tapper_C" _returnvalue))
  (bind _output_get (set `self.NewVar` _returnvalue_3))
  (`UserWidget.AddToViewport` _output_get 0))

(event `EnhancedInput|/Game/input/IA_Tapper`
  (params (ActionValue :type Boolean) (ElapsedSeconds :type "Float (double-precision)") (TriggeredSeconds :type "Float (double-precision)") (InputAction :type "InputAction Object Reference" :default "/Game/input/IA_Tapper.IA_Tapper"))
  (:`Started`
    (`self.Tapper`)))

(fn `UserConstructionScript`
  (`parent.UserConstructionScript`))